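; BP_GamePlayerController is the player controller that routes Enhanced Input to the possessed pawn.
; BeginPlay adds the IMC_Game mapping context, and IA_Move drives movement input along fixed world X and Y axes.
; Pick-up and bat inputs call Interact and BecomeBat on BP_PlayerCharacter through a GetContoller cast helper.
; Rat and ogre inputs have empty handlers.
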(event Input|EnhancedActionEvents|EnhancedInputActionIA_PickUp
  (params (ActionValue :type Boolean) (ElapsedSeconds :type Float%20%28double-precision%29) (TriggeredSeconds :type Float%20%28double-precision%29) (InputAction :type Input%20Action%20Object%20Reference :default "/Game/Game/Input/Actions/IA_PickUp.IA_PickUp"))
  (:Started
    (bind _asbp_top_down_character (Utilities|GetContoller))
    (Default|Interact _asbp_top_down_character)))

(event Input|EnhancedActionEvents|EnhancedInputActionIA_Rat
  (params (ActionValue :type Boolean) (ElapsedSeconds :type Float%20%28double-precision%29) (TriggeredSeconds :type Float%20%28double-precision%29) (InputAction :type Input%20Action%20Object%20Reference :default "/Game/Game/Input/Actions/IA_Rat.IA_Rat")))

(event Input|EnhancedActionEvents|EnhancedInputActionIA_Bat
  (params (ActionValue :type Boolean) (ElapsedSeconds :type Float%20%28double-precision%29) (TriggeredSeconds :type Float%20%28double-precision%29) (InputAction :type Input%20Action%20Object%20Reference :default "/Game/Game/Input/Actions/IA_Bat.IA_Bat")))

(event Input|EnhancedActionEvents|EnhancedInputActionIA_Ogre
  (params (ActionValue :type Boolean) (ElapsedSeconds :type Float%20%28double-precision%29) (TriggeredSeconds :type Float%20%28double-precision%29) (InputAction :type Input%20Action%20Object%20Reference :default "/Game/Game/Input/Actions/IA_Ogre.IA_Ogre")))

(event Input|EnhancedActionEvents|EnhancedInputActionIA_Move
  (params (ActionValue :type Vector%202D%20Structure) (ElapsedSeconds :type Float%20%28double-precision%29) (TriggeredSeconds :type Float%20%28double-precision%29) (InputAction :type Input%20Action%20Object%20Reference :default "/Game/Game/Input/Actions/IA_Move.IA_Move"))
  (bind _returnvalue (Pawn|GetControlledPawn))
  ;[1 1 1] Player Movement
  (Pawn|Input|AddMovementInput _returnvalue "0.000000,1.000000,0.000000" (.x ActionValue) false)
  (Pawn|Input|AddMovementInput _returnvalue "1.000000,0.000000,0.000000" (.y ActionValue) false))

(event Input|EnhancedActionEvents|EnhancedInputActionIA_Bat
  (params (ActionValue :type Boolean) (ElapsedSeconds :type Float%20%28double-precision%29) (TriggeredSeconds :type Float%20%28double-precision%29) (InputAction :type Input%20Action%20Object%20Reference :default "/Game/Game/Input/Actions/IA_Bat.IA_Bat"))
  (:Started
    (bind _asbp_top_down_character (Utilities|GetContoller))
    (Default|BecomeBat _asbp_top_down_character)))

(event EventBeginPlay
  (bind _returnvalue (Game|GetPlayerController 0))
  (bind _returnvalue_2 (PlayerController|LocalPlayerSubsystems|GetEnhancedInputLocalPlayerSubsystem _returnvalue))
  ;[1 1 1] Add Mapping Context
  (Utilities|IsValid _returnvalue_2
    (:Is%20Valid
      (Input|AddMappingContext _returnvalue_2 "/Game/Game/Input/IMC_Game.IMC_Game" 0 "(bIgnoreAllPressedKeysUntilRelease=True,bForceImmediately=False,bNotifyUserSettings=False)"))))

(event EventTick
  (params (DeltaSeconds :type Float%20%28single-precision%29)))

(fn ConstructionScript)