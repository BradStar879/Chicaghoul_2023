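; Blueprint function library of helpers for the ingredient enum used by a potion-themed game.
; Switches map each ingredient to its actor class and texture, and flag Cauldron, Pumpkin and Flask as containers.
; GetAllIngredients loops over the enum past None, splitting entries into container and non-container lists.
; GetUniqueIngredients draws random non-container ingredients without repeats by removing each pick from that list.
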(fn IngredienttoClass
  (params (Ingredient :type EIngredient%20Enum :default "NewEnumerator0"))
  (switch Utilities|FlowControl|Switch|SwitchonEIngredient Ingredient
    (:NewEnumerator0
      (return 0))
    (:NewEnumerator1
      (return "/Game/Game/Blueprints/Actors/Ingredients/BP_Cauldron.BP_Cauldron_C"))
    (:NewEnumerator2
      (return "/Game/Game/Blueprints/Actors/Ingredients/BP_Pumpkin.BP_Pumpkin_C"))
    (:NewEnumerator3
      (return "/Game/Game/Blueprints/Actors/Ingredients/BP_Flask.BP_Flask_C"))
    (:NewEnumerator4
      (return "/Game/Game/Blueprints/Actors/Ingredients/BP_NewtEye.BP_NewtEye_C"))
    (:NewEnumerator5
      (return "/Game/Game/Blueprints/Actors/Ingredients/BP_FrogTongue.BP_FrogTongue_C"))
    (:NewEnumerator6
      (return "/Game/Game/Blueprints/Actors/Ingredients/BP_PixieWings.BP_PixieWings_C"))
    (:NewEnumerator7
      (return "/Game/Game/Blueprints/Actors/Ingredients/BP_LizardLeg.BP_LizardLeg_C"))
    (:NewEnumerator8
      (return "/Game/Game/Blueprints/Actors/Ingredients/BP_DragonClaw.BP_DragonClaw_C"))))

(fn IngredientIsContainer
  (params (Ingredient :type EIngredient%20Enum :default "NewEnumerator0"))
  (switch Utilities|FlowControl|Switch|SwitchonEIngredient Ingredient
    (:NewEnumerator0
      _)
    (:NewEnumerator1
      (return true))
    (:NewEnumerator2
      (return true))
    (:NewEnumerator3
      (return true))
    (:NewEnumerator4
      _)
    (:NewEnumerator5
      _)
    (:NewEnumerator6
      _)
    (:NewEnumerator7
      _)
    (:NewEnumerator8
      _))
  (return false))

(fn GetAllIngredients
  (for _index (range 1 (- (|GetNumEnumEntries) 1))
    (if (CallFunction|IngredientIsContainer (Utilities|Enum|ByteToEnumEIngredient (Math|Conversions|ToByte(Integer) _index)))
      (Utilities|Array|Add (LocalVariables|GetContainerIngredientsTemp) (Utilities|Enum|ByteToEnumEIngredient (Math|Conversions|ToByte(Integer) _index)))
      (else
        (Utilities|Array|Add (LocalVariables|GetNonContainerIngredientsTemp) (Utilities|Enum|ByteToEnumEIngredient (Math|Conversions|ToByte(Integer) _index))))))
  (return (LocalVariables|GetNonContainerIngredientsTemp) (LocalVariables|GetContainerIngredientsTemp)))

(fn GetUniqueIngredients
  (params (Number%20Of%20Elements :type Integer))
  (bind _noncontaineringredients (CallFunction|GetAllIngredients))
  (LocalVariables|SetNonContainerIngredients _noncontaineringredients)
  (for _index (range 1 Number%20Of%20Elements)
    (bind _output_get (LocalVariables|SetTempIngredient (.OutItem (Utilities|Array|Random (LocalVariables|GetNonContainerIngredients)))))
    (Utilities|Array|Add (LocalVariables|GetChosenIngredients) _output_get)
    (Utilities|Array|RemoveItem (LocalVariables|GetNonContainerIngredients) _output_get))
  (return (LocalVariables|GetChosenIngredients)))

(fn GetIngredientTexturefromEnum
  (params (Ingredient :type EIngredient%20Enum :default "NewEnumerator0"))
  (switch Utilities|FlowControl|Switch|SwitchonEIngredient Ingredient
    (:NewEnumerator0
      (return 0))
    (:NewEnumerator1
      (return "/Game/Game/UI/MainLevel/Icons/Cauldron.Cauldron"))
    (:NewEnumerator2
      (return "/Game/Game/UI/MainLevel/Icons/Pumpkin.Pumpkin"))
    (:NewEnumerator3
      (return "/Game/Game/UI/MainLevel/Icons/Flask.Flask"))
    (:NewEnumerator4
      (return "/Game/Game/UI/MainLevel/Icons/Newt_Eye_Placeholder.Newt_Eye_Placeholder"))
    (:NewEnumerator5
      (return "/Game/Game/UI/MainLevel/Icons/Frog_Tongue.Frog_Tongue"))
    (:NewEnumerator6
      (return "/Game/Game/UI/MainLevel/Icons/Pixie_Wings.Pixie_Wings"))
    (:NewEnumerator7
      (return "/Game/Game/UI/MainLevel/Icons/Lizard_Leg.Lizard_Leg"))
    (:NewEnumerator8
      (return "/Game/Game/UI/MainLevel/Icons/Dragon_Claw.Dragon_Claw"))))