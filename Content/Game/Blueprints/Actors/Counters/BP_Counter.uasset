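; BP_Counter is a counter actor that holds an ingredient pickup above it, either one placed on it or one it spawns as a source.
; SetPickUp attaches a given ingredient with collision disabled, while SetSourcePickUp spawns the pickup class mapped from an ingredient and flags the counter as a source.
; RemovePickUp releases the stored reference only on non-source counters, and ClearCounter destroys any held ingredient and resets the source flag.
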(event EventBeginPlay)

(event Collision|EventActorBeginOverlap
  (params (OtherActor :type Actor%20Object%20Reference)))

(event EventTick
  (params (DeltaSeconds :type Float%20%28single-precision%29)))

(fn ConstructionScript)

(fn SetPickUp
  (params (Ingredient%20Actor :type BP%20Pick%20Up%20Object%20Reference))
  (Variables|Default|SetSource false)
  (bind _output_get (Variables|Default|SetIngredientActor Ingredient%20Actor))
  (Collision|SetActorEnableCollision _output_get false)
  (Transformation|AttachActorToActor _output_get self "None" "KeepRelative" "KeepRelative" "KeepRelative" true)
  (Transformation|AddLocalOffset (Variables|/Script/Engine.Actor|GetRootComponent _output_get) "0.000000,0.000000,83.000000" false false))

(fn SetSourcePickUp
  (params (Ingredient :type EIngredient%20Enum :default "NewEnumerator0"))
  (Variables|Default|SetSource true)
  (bind _returnvalue (Game|SpawnActorfromClass (CallFunction|IngredienttoClass Ingredient) (Transformation|GetActorTransform) "Undefined" "MultiplyWithRoot" 0 0))
  (bind _asbp_pick_up (Utilities|Casting|CastToBP_PickUp _returnvalue))
  (Variables|Default|SetIngredientActor _asbp_pick_up)
  (Transformation|AddLocalOffset (Variables|/Script/Engine.Actor|GetRootComponent _asbp_pick_up) "0.000000,0.000000,83.000000" false false))

(fn RemovePickUp
  (if (not (Variables|Default|GetSource))
    (Variables|Default|SetIngredientActor 0)))

(fn ClearCounter
  (if (Utilities|IsValid (Variables|Default|GetIngredientActor))
    (Actor|DestroyActor (Variables|Default|GetIngredientActor))
    (Variables|Default|SetIngredientActor 0)
    (Variables|Default|SetSource false)))