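; Bar counter actor that spawns a customer with a random brew order and judges the brew handed to it.
; Each order is a random container plus three unique ingredients, shown with a countdown on the customer's widgets and ticked down while active.
; A brew matches by length and contents regardless of order, scoring by level and remaining time.
; A wrong brew or timeout sends the customer away and costs a life through BP_MainGameMode.
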(event EventBeginPlay
  (Variables|Default|SetInitial%20Wait%20Timer 6e+01))

(event Collision|EventActorBeginOverlap
  (params (OtherActor :type Actor%20Object%20Reference)))

(event EventTick
  (params (DeltaSeconds :type Float%20%28single-precision%29))
  (CallFunction|CheckWaitTimer DeltaSeconds))

(fn ConstructionScript)

(fn CreateBrewOrder
  (Variables|Default|SetOrderActive true)
  (Variables|Default|SetWait%20Timer (Variables|Default|GetInitial%20Wait%20Timer))
  (bind _containeringredients (CallFunction|GetAllIngredients))
  (Utilities|Array|Add (LocalVariables|GetOrder) (.OutItem (Utilities|Array|Random _containeringredients)))
  (bind _ingredients (CallFunction|GetUniqueIngredients 3))
  (for _array_element _ingredients
    (Utilities|Array|Add (LocalVariables|GetOrder) (Utilities|Enum|ByteToEnumEIngredient _array_element)))
  (Variables|Default|SetBrewOrder (LocalVariables|GetOrder)))

(fn CheckOrder
  (params (BrewGiven :type Array%20of%20Bytes) (Level%20Number :type Integer))
  (if (Variables|Default|GetOrderActive)
    (LocalVariables|SetBrewGivenTemp BrewGiven)
    (bind _asbp_main_game_mode (Utilities|Casting|CastToBP_MainGameMode (Game|GetGameMode)))
    (if (== (Utilities|Array|Length BrewGiven) (Utilities|Array|Length (Variables|Default|GetBrewOrder)))
      (for _array_element (Variables|Default|GetBrewOrder)
        (if (not (Utilities|Array|ContainsItem (LocalVariables|GetBrewGivenTemp) _array_element))
          (Variables|Default|SetOrderActive false)
          (Default|SpeedNextCustomerifBarEmpty _asbp_main_game_mode)
          (CallFunction|FailCustomer)
          (return false true 0)))
      (Default|Leave (Variables|Default|GetCustomer))
      (Variables|Default|SetCustomer 0)
      (Variables|Default|SetOrderActive false)
      (Default|SpeedNextCustomerifBarEmpty _asbp_main_game_mode)
      (Default|IncrementCustomersServed _asbp_main_game_mode)
      (bind _score_to_add (CallFunction|CalculateOrderScore Level%20Number (Variables|Default|GetInitial%20Wait%20Timer) (Variables|Default|GetWait%20Timer)))
      (return true true _score_to_add)
      (else
        (Variables|Default|SetOrderActive false)
        (Default|SpeedNextCustomerifBarEmpty _asbp_main_game_mode)
        (CallFunction|FailCustomer)
        (return false true 0)))
    (else
      (return false false 0))))

(fn SpawnCustomer
  (bind _breworder (Variables|Default|GetBrewOrder))
  (bind _returnvalue (Game|SpawnActorfromClass "/Game/Game/Blueprints/Actors/BP_Customer.BP_Customer_C" (Transformation|GetActorTransform) "Undefined" "MultiplyWithRoot" 0 0))
  (bind _output_get (Variables|Default|SetCustomer _returnvalue))
  (bind _aswait_timer (Utilities|Casting|CastToWaitTimer (UserInterface|GetUserWidgetObject (Variables|/Game/Game/Blueprints/Actors/BP_Customer.BP_Customer_C|GetTimer%20Widget _output_get))))
  (bind _output_get_2 (Variables|Default|SetWait%20Timer%20Widget _aswait_timer))
  (Variables|/Game/Game/UI/MainLevel/WaitTimer.WaitTimer_C|SetInitial%20Time _output_get_2 (Variables|Default|GetInitial%20Wait%20Timer))
  (Transformation|AddActorLocalOffset _output_get "0.000000,-100.000000,50.000000" false false)
  (Transformation|AddActorLocalRotation _output_get "0.000000,90.000000,0.000000" false false)
  (CallFunction|CreateBrewOrder)
  (bind _asorder_display (Utilities|Casting|CastToOrderDisplay (UserInterface|GetUserWidgetObject (Variables|/Game/Game/Blueprints/Actors/BP_Customer.BP_Customer_C|GetOrder%20Widget (Variables|Default|GetCustomer)))))
  (Default|SetOrderUI _asorder_display (Utilities|Array|Get(acopy) _breworder) (Utilities|Array|Get(acopy) _breworder 1) (Utilities|Array|Get(acopy) _breworder 2) (Utilities|Array|Get(acopy) _breworder 3)))

(fn FailCustomer
  (Variables|Default|SetOrderActive false)
  (Default|Leave (Variables|Default|GetCustomer))
  (bind _asbp_main_game_mode (Utilities|Casting|CastToBP_MainGameMode (Game|GetGameMode)))
  (Default|LoseLife _asbp_main_game_mode))

(fn CheckWaitTimer
  (params (InputPin :type Float%20%28single-precision%29))
  (if (Variables|Default|GetOrderActive)
    (bind _output_get (Variables|Default|SetWait%20Timer (- (Variables|Default|GetWait%20Timer) InputPin)))
    (if (<= _output_get 0.0)
      (CallFunction|FailCustomer)
      (else
        (Default|UpdateTime (Variables|Default|GetWait%20Timer%20Widget) (Variables|Default|GetWait%20Timer))))))

(fn CalculateOrderScore
  (params (Level%20Number :type Integer) (Initial%20Time :type Float%20%28double-precision%29) (Remaining%20Time :type Float%20%28double-precision%29))
  (return (Math|Float|Truncate (* (* (* Level%20Number 1.5) (/ Remaining%20Time Initial%20Time)) 1e+03))))