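; BP_PickUp is an ingredient pickup actor that can act as a container for other ingredients, based on its Type.
; AddIngredientToContainer stores the ingredient in hand in IngredientsInContainer only if this pickup is a container, that ingredient is not one, and it is not already stored.
; It returns whether the add succeeded.
; The event graph and construction script have no active logic.
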(event EventBeginPlay)

(event Collision|EventActorBeginOverlap
  (params (OtherActor :type Actor%20Object%20Reference)))

(event EventTick
  (params (DeltaSeconds :type Float%20%28single-precision%29)))

(fn ConstructionScript)

(fn AddIngredienttoContainer
  (params (Ingredient%20In%20Hand :type EIngredient%20Enum :default "None"))
  (if (and (not (CallFunction|IngredientIsContainer Ingredient%20In%20Hand)) (and (CallFunction|IngredientIsContainer (Variables|Default|GetType)) (not (Utilities|Array|ContainsItem (Variables|Default|GetIngredientsInContainer) Ingredient%20In%20Hand)))) ; Is ingredient valid container
    (Utilities|Array|Add (Variables|Default|GetIngredientsInContainer) Ingredient%20In%20Hand)
    (return true)
    (else
      (return false))))