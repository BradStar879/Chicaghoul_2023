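; Player character for a potion-serving game, able to transform between Human and Bat, Rat or Ogre.
; Overlaps track the nearby counter, trash or bar counter, which Interact uses to carry, combine, discard or serve ingredients, with GameMode scoring orders.
; Ogre-only counters work only for the Ogre, other counters only for other forms.
; Forms change scale or height; Bat holds its altitude on Tick and toggles shelf materials between opaque and transparent.
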(event EventBeginPlay
  (bind _asbp_main_game_mode (Utilities|Casting|CastToBP_MainGameMode (Game|GetGameMode)))
  (Variables|Default|SetGame%20Mode _asbp_main_game_mode))

(event Collision|EventActorBeginOverlap
  (params (OtherActor :type Actor%20Object%20Reference))
  (bind _asbp_counter (Utilities|Casting|CastToBP_Counter OtherActor)
    (:then
      (Variables|Default|SetNearbyInteraction _asbp_counter))
    (:CastFailed
      (bind _asbp_trash (Utilities|Casting|CastToBP_Trash OtherActor)
        (:then
          (Variables|Default|SetNearbyInteraction _asbp_trash))
        (:CastFailed
          (bind _asbp_bar_counter (Utilities|Casting|CastToBP_BarCounter OtherActor))
          (Variables|Default|SetNearbyInteraction _asbp_bar_counter))))))

(event Collision|EventActorEndOverlap
  (params (OtherActor :type Actor%20Object%20Reference))
  (if (== OtherActor (Variables|Default|GetNearbyInteraction))
    (Variables|Default|SetNearbyInteraction 0)))

(event EventTick
  (params (DeltaSeconds :type Float%20%28single-precision%29))
  (bind _returnvalue (Transformation|GetActorTransform))
  (switch Utilities|FlowControl|Switch|SwitchonETransformState (Variables|Default|GetTransform%20State)
    (:NewEnumerator2
      (Transformation|SetActorLocation (Math|Vector|MakeVector (.x (.location _returnvalue)) (.y (.location _returnvalue)) 4.4e+02) false false))))

(fn ConstructionScript)

(fn Interact
  (bind _asbp_counter (Utilities|Casting|CastToBP_Counter (Variables|Default|GetNearbyInteraction))
    (:then
      (CallFunction|InteractwithCounter _asbp_counter))
    (:CastFailed
      (Utilities|Casting|CastToBP_Trash (Variables|Default|GetNearbyInteraction)
        (:then
          (CallFunction|EmptyHand))
        (:CastFailed
          (bind _asbp_bar_counter (Utilities|Casting|CastToBP_BarCounter (Variables|Default|GetNearbyInteraction)))
          (CallFunction|InteractwithBarCounter _asbp_bar_counter))))))

(fn EmptyHand
  (if (Utilities|IsValid (Variables|Default|GetIngredient%20In%20Hand))
    (Actor|DestroyActor (Variables|Default|GetIngredient%20In%20Hand))
    (Variables|Default|SetIngredient%20In%20Hand 0)))

(fn PutinHand
  (params (Counter :type BP%20Counter%20Object%20Reference))
  (bind _ingredientactor (Variables|/Game/Game/Blueprints/Actors/Counters/BP_Counter.BP_Counter_C|GetIngredientActor Counter))
  (if (Variables|/Game/Game/Blueprints/Actors/Counters/BP_Counter.BP_Counter_C|GetSource Counter)
    (bind _returnvalue (Game|SpawnActorfromClass (CallFunction|IngredienttoClass (Variables|/Game/Game/Blueprints/Actors/Ingredients/BP_PickUp.BP_PickUp_C|GetType _ingredientactor)) (Transformation|GetActorTransform) "Undefined" "MultiplyWithRoot" 0 0))
    (LocalVariables|SetIngredient%20Actor _returnvalue)
    (else
      (LocalVariables|SetIngredient%20Actor _ingredientactor)))
  (Collision|SetActorEnableCollision (LocalVariables|GetIngredient%20Actor) false)
  (Transformation|AttachActorToActor (LocalVariables|GetIngredient%20Actor) self "None" "SnapToTarget" "SnapToTarget" "SnapToTarget" true)
  (bind _asbp_pick_up (Utilities|Casting|CastToBP_PickUp (LocalVariables|GetIngredient%20Actor)))
  (Variables|Default|SetIngredient%20In%20Hand _asbp_pick_up))

(fn InteractwithCounter
  (params (Counter :type BP%20Counter%20Object%20Reference))
  (if (== (Variables|/Game/Game/Blueprints/Actors/Counters/BP_Counter.BP_Counter_C|GetOgre%20Only Counter) (Utilities|Enum|Equal(Enum) (Variables|Default|GetTransform%20State) "NewEnumerator1"))
    (if (Utilities|IsValid (Variables|/Game/Game/Blueprints/Actors/Counters/BP_Counter.BP_Counter_C|GetIngredientActor Counter)) ; Ingredient on counter
      (if (Utilities|IsValid (Variables|Default|GetIngredient%20In%20Hand)) ; Ingredient in hand
        (bind _canputingredient (Default|AddIngredienttoContainer (Variables|/Game/Game/Blueprints/Actors/Counters/BP_Counter.BP_Counter_C|GetIngredientActor Counter) (Variables|/Game/Game/Blueprints/Actors/Ingredients/BP_PickUp.BP_PickUp_C|GetType (Variables|Default|GetIngredient%20In%20Hand))))
        (if _canputingredient
          (CallFunction|EmptyHand))
        (else
          (CallFunction|PutinHand Counter)
          (Default|RemovePickUp Counter)))
      (elif (Utilities|IsValid (Variables|Default|GetIngredient%20In%20Hand)) ; Ingredient in hand
        (Default|SetPickUp Counter (Variables|Default|GetIngredient%20In%20Hand))
        (Variables|Default|SetIngredient%20In%20Hand 0)))))

(fn InteractwithBarCounter
  (params (Bar%20Counter :type BP%20Bar%20Counter%20Object%20Reference))
  (bind _ingredient_in_hand (Variables|Default|GetIngredient%20In%20Hand))
  (if (Utilities|IsValid _ingredient_in_hand)
    (if (CallFunction|IngredientIsContainer (Variables|/Game/Game/Blueprints/Actors/Ingredients/BP_PickUp.BP_PickUp_C|GetType _ingredient_in_hand))
      (bind (_correctorder _remove_from_hand _score_to_add) (Default|CheckOrder Bar%20Counter (Variables|/Game/Game/Blueprints/Actors/Ingredients/BP_PickUp.BP_PickUp_C|GetIngredientsInContainer (Variables|Default|GetIngredient%20In%20Hand)) (Variables|/Game/Game/Blueprints/GameModes/BP_MainGameMode.BP_MainGameMode_C|GetLevel%20Number (Variables|Default|GetGame%20Mode))))
      (Default|AddScore (Variables|Default|GetGame%20Mode) _score_to_add)
      (if _remove_from_hand
        (CallFunction|EmptyHand))
      (if _correctorder
        (Default|CheckWinLevel (Variables|Default|GetGame%20Mode))))))

(fn BecomeBat
  (if (Variables|Default|GetCan%20Transform)
    (switch Utilities|FlowControl|Switch|SwitchonETransformState (Variables|Default|GetTransform%20State)
      (:NewEnumerator0
        (Variables|Default|SetTransform%20State "NewEnumerator2")
        (LocalVariables|SetMaterial%20to%20Set "/Game/Game/Materials/M_WoodCounter.M_WoodCounter"))
      (:NewEnumerator2
        (CallFunction|BecomeHuman)
        (LocalVariables|SetMaterial%20to%20Set "/Game/Game/Materials/M_WoodCounterTransparent.M_WoodCounterTransparent")))
    (bind _outactors (Actor|GetAllActorsOfClass "/Game/Game/Blueprints/Actors/Counters/BP_Shelf.BP_Shelf_C"))
    (for _array_element _outactors
      (Rendering|Material|SetMaterial (Variables|/Game/Game/Blueprints/Actors/Counters/BP_Counter.BP_Counter_C|GetStaticMesh _array_element) 0 (LocalVariables|GetMaterial%20to%20Set)))))

(fn BecomeRat
  (bind _returnvalue (Transformation|GetActorTransform))
  (if (Variables|Default|GetCan%20Transform)
    (switch Utilities|FlowControl|Switch|SwitchonETransformState (Variables|Default|GetTransform%20State)
      (:NewEnumerator0
        (Variables|Default|SetTransform%20State "NewEnumerator3")
        (Transformation|SetActorRelativeScale3D "0.250000,0.250000,0.250000")
        (Transformation|SetActorLocation (Math|Vector|MakeVector (.x (.location _returnvalue)) (.y (.location _returnvalue)) 30.6) false false))
      (:NewEnumerator3
        (CallFunction|BecomeHuman)))))

(fn BecomeOgre
  (bind _returnvalue (Transformation|GetActorTransform))
  (if (Variables|Default|GetCan%20Transform)
    (switch Utilities|FlowControl|Switch|SwitchonETransformState (Variables|Default|GetTransform%20State)
      (:NewEnumerator0
        (Variables|Default|SetTransform%20State "NewEnumerator1")
        (Transformation|SetActorRelativeScale3D "1.500000,1.500000,1.500000")
        (Transformation|SetActorLocation (Math|Vector|MakeVector (.x (.location _returnvalue)) (.y (.location _returnvalue)) 146.2) false false))
      (:NewEnumerator1
        (CallFunction|BecomeHuman)))))

(fn BecomeHuman
  (bind _returnvalue (Transformation|GetActorTransform))
  (Variables|Default|SetTransform%20State "NewEnumerator0")
  (Transformation|SetActorLocation (Math|Vector|MakeVector (.x (.location _returnvalue)) (.y (.location _returnvalue)) 98.0) false false)
  (Transformation|SetActorRelativeScale3D "1.000000,1.000000,1.000000"))