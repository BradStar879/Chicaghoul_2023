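; Main game mode for a bar service game played over numbered nights, tracking score, lives and customers served.
; Tick either spawns timed customers at free bar counters or counts down to the next night behind a night-number widget.
; Each night clears and randomly restocks ingredient counters, with spawn interval and customer count tuned for six nights.
; Losing a life adds a replacement customer, or shows the lose screen at zero.
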(event EventBeginPlay
  (Variables|Default|SetScore 0)
  (bind _returnvalue (UserInterface|CreateWidget "/Game/Game/UI/MainLevel/NightCounter.NightCounter_C"))
  (Variables|Default|SetNight%20Counter%20UI _returnvalue)
  (bind _returnvalue_2 (UserInterface|CreateWidget "/Game/Game/UI/MainLevel/MainUI.MainUI_C"))
  (bind _output_get (Variables|Default|SetMain%20UI _returnvalue_2))
  (Default|SetScore _output_get)
  (UserInterface|Viewport|AddtoViewport _output_get 0))

(event EventTick
  (params (DeltaSeconds :type Float%20%28single-precision%29))
  (if (Variables|Default|GetLevel%20Active)
    (CallFunction|CustomerSpawnCheck DeltaSeconds)
    (elif (Variables|Default|GetLoad%20Next%20Level)
      (CallFunction|NewLevelSequence DeltaSeconds))))

(fn ConstructionScript)

(fn SetStartingIngredientsonCounters
  (bind (_noncontaineringredients _containeringredients) (CallFunction|GetAllIngredients))
  (for _array_element _noncontaineringredients
    (Utilities|Array|Add (LocalVariables|GetIngredient%20Types) _array_element))
  (for _array_element_2 _containeringredients
    (Utilities|Array|Add (LocalVariables|GetIngredient%20Types) _array_element_2))
  (bind _outactors (Actor|GetAllActorsOfClass "/Game/Game/Blueprints/Actors/Counters/BP_Counter.BP_Counter_C"))
  (LocalVariables|SetAll%20Counters _outactors)
  (for _array_element_3 (LocalVariables|GetIngredient%20Types)
    (bind _asbp_counter (Utilities|Casting|CastToBP_Counter (.OutItem (Utilities|Array|Random (LocalVariables|GetAll%20Counters)))))
    (Default|SetSourcePickUp _asbp_counter _array_element_3)
    (Utilities|Array|RemoveItem (LocalVariables|GetAll%20Counters) _asbp_counter)))

(fn SpawnCustomeratRandomCounter
  (bind _outactors (Actor|GetAllActorsOfClass "/Game/Game/Blueprints/Actors/Counters/BP_BarCounter.BP_BarCounter_C"))
  (for _array_element _outactors
    (if (not (Variables|/Game/Game/Blueprints/Actors/Counters/BP_BarCounter.BP_BarCounter_C|GetOrderActive _array_element))
      (Utilities|Array|Add (LocalVariables|GetOpen%20Bar%20Counters) _array_element)))
  (Default|SpawnCustomer (.OutItem (Utilities|Array|Random (LocalVariables|GetOpen%20Bar%20Counters))))
  (Variables|Default|SetTime%20Since%20Last%20Customer 0.0)
  (Math|Integer|DecrementInt (Variables|Default|GetCustomers%20to%20Spawn)))

(fn CustomerSpawnCheck
  (params (Delta%20Time :type Float%20%28double-precision%29))
  (if (and (> (Variables|Default|GetCustomers%20to%20Spawn) 0) (Variables|Default|GetLevel%20Active))
    (bind _output_get (Variables|Default|SetTime%20Since%20Last%20Customer (+ Delta%20Time (Variables|Default|GetTime%20Since%20Last%20Customer))))
    (if (>= _output_get (Variables|Default|GetTime%20Between%20Customers%20Spawn))
      (bind _outactors (Actor|GetAllActorsOfClass "/Game/Game/Blueprints/Actors/Counters/BP_BarCounter.BP_BarCounter_C"))
      (bind _array_element (Utilities|Array|ForEachLoopwithBreak _outactors :!label _label)
        (:LoopBody
          (if (not (Variables|/Game/Game/Blueprints/Actors/Counters/BP_BarCounter.BP_BarCounter_C|GetOrderActive _array_element))
            (LocalVariables|SetAvailable%20Counter true)
            (goto _label Break)))
        (:Completed
          (if (LocalVariables|GetAvailable%20Counter)
            (CallFunction|SpawnCustomeratRandomCounter)
            (else
              (Variables|Default|SetTime%20Since%20Last%20Customer (- (Variables|Default|GetTime%20Since%20Last%20Customer) 7.0)))))))))

(fn BeginLevel
  (params (Level%20Number :type Integer))
  (Widget|RemovefromParent (Variables|Default|GetNight%20Counter%20UI))
  (Variables|Default|SetNight%20Text%20Active false)
  (Variables|Default|SetTime%20Until%20Next%20Level 7.0)
  (Variables|Default|SetLevel%20Active true)
  (Variables|Default|SetLoad%20Next%20Level false)
  (bind _output_get (Variables|Default|SetLives 3))
  (Default|SetLives (Variables|Default|GetMain%20UI) _output_get)
  (Variables|Default|SetTime%20Since%20Last%20Customer 0.0)
  (CallFunction|ClearCounters)
  (CallFunction|SetStartingIngredientsonCounters)
  (CallFunction|SpawnCustomeratRandomCounter)
  (switch int Level%20Number
    (:1
      (Variables|Default|SetTime%20Between%20Customers%20Spawn 45.0)
      (Variables|Default|SetCustomers%20to%20Spawn 1))
    (:2
      (Variables|Default|SetTime%20Between%20Customers%20Spawn 4e+01)
      (Variables|Default|SetCustomers%20to%20Spawn 3))
    (:3
      (Variables|Default|SetTime%20Between%20Customers%20Spawn 35.0)
      (Variables|Default|SetCustomers%20to%20Spawn 4))
    (:4
      (Variables|Default|SetTime%20Between%20Customers%20Spawn 3e+01)
      (Variables|Default|SetCustomers%20to%20Spawn 5))
    (:5
      (Variables|Default|SetTime%20Between%20Customers%20Spawn 25.0)
      (Variables|Default|SetCustomers%20to%20Spawn 6))
    (:6
      (Variables|Default|SetTime%20Between%20Customers%20Spawn 2e+01)
      (Variables|Default|SetCustomers%20to%20Spawn 7))))

(fn CheckWinLevel
  (bind _customer_at_a_counter (CallFunction|IsCustomeratACounter))
  (if (and (not _customer_at_a_counter) (== (Variables|Default|GetCustomers%20to%20Spawn) 0))
    (Variables|Default|SetLevel%20Active false)
    (Variables|Default|SetLoad%20Next%20Level true)
    (Development|PrintText "You Win!")))

(fn IsCustomeratACounter
  (bind _outactors (Actor|GetAllActorsOfClass "/Game/Game/Blueprints/Actors/Counters/BP_BarCounter.BP_BarCounter_C"))
  (for _array_element _outactors
    (if (Variables|/Game/Game/Blueprints/Actors/Counters/BP_BarCounter.BP_BarCounter_C|GetOrderActive _array_element)
      (return true)))
  (return false))

(fn NewLevelSequence
  (params (Delta%20Time :type Float%20%28double-precision%29))
  (bind _output_get (Variables|Default|SetTime%20Until%20Next%20Level (- (Variables|Default|GetTime%20Until%20Next%20Level) Delta%20Time)))
  (if (<= _output_get 0.0)
    (Variables|Default|SetNight%20Text%20Active false)
    (Variables|Default|SetTime%20Until%20Next%20Level 5.0)
    (CallFunction|BeginLevel (Variables|Default|GetLevel%20Number))
    (else
      (CallFunction|DisplayNightText))))

(fn ClearCounters
  (bind _outactors (Actor|GetAllActorsOfClass "/Game/Game/Blueprints/Actors/Counters/BP_Counter.BP_Counter_C"))
  (for _array_element _outactors
    (Default|ClearCounter _array_element)))

(fn LoseLife
  (bind _result (Math|Integer|DecrementInt (Variables|Default|GetLives))
    (:%20%20
      (Default|SetLives (Variables|Default|GetMain%20UI) _result)
      (if (== _result 0)
        (bind _returnvalue (UserInterface|CreateWidget "/Game/Game/UI/MainLevel/LoseScreen.LoseScreen_C"))
        (Default|SetStats _returnvalue (Variables|Default|GetLevel%20Number) (Variables|Default|GetCustomers%20Served))
        (UserInterface|Viewport|AddtoViewport _returnvalue 0)
        (Variables|Default|SetLevel%20Active false)
        (Variables|/Script/Engine.PlayerController|SetbShowMouseCursor (Game|GetPlayerController 0) true)
        (else
          (Math|Integer|IncrementInt (Variables|Default|GetCustomers%20to%20Spawn)))))))

(fn DisplayNightText
  (bind _night_counter_ui (Variables|Default|GetNight%20Counter%20UI))
  (if (not (Variables|Default|GetNight%20Text%20Active))
    (Variables|Default|SetNight%20Text%20Active true)
    (bind _result (Math|Integer|IncrementInt (Variables|Default|GetLevel%20Number))
      (:%20%20
        (if (<= _result 6)
          (UserInterface|Viewport|AddtoViewport _night_counter_ui 0)
          (Default|SetNightNumber _night_counter_ui (Variables|Default|GetLevel%20Number)))))))

(fn SpeedNextCustomerifBarEmpty
  (bind _customer_at_a_counter (CallFunction|IsCustomeratACounter))
  (if (not _customer_at_a_counter)
    (Variables|Default|SetTime%20Since%20Last%20Customer (Math|Float|Max(Float) (- (Variables|Default|GetTime%20Between%20Customers%20Spawn) 5.0) (Variables|Default|GetTime%20Since%20Last%20Customer)))))

(fn IncrementCustomersServed
  (Math|Integer|IncrementInt (Variables|Default|GetCustomers%20Served)))

(fn AddScore
  (params (Score%20To%20Add :type Integer))
  (bind _output_get (Variables|Default|SetScore (+ Score%20To%20Add (Variables|Default|GetScore))))
  (Default|SetScore (Variables|Default|GetMain%20UI) _output_get))